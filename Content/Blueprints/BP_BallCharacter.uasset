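; BP_BallCharacter is a player-controlled rolling ball that faux-tilts the view as it moves.
; IA_Tilt applies torque to the physics sphere and switches angular damping off while held, restoring it on release to slow the spin.
; Tick eases spring arm and BP_GoodSky rotation toward the tilt input, and lengthens the arm with speed.
; A toggleable arrow shows velocity direction and speed; an unconnected sky-sphere lookup never runs.
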(event Input|EnhancedActionEvents|EnhancedInputActionIA_Tilt
  (params (ActionValue :type Vector%202D%20Structure) (ElapsedSeconds :type Float%20%28double-precision%29) (TriggeredSeconds :type Float%20%28double-precision%29) (InputAction :type Input%20Action%20Object%20Reference :default "/Game/Blueprints/Input/Actions/IA_Tilt.IA_Tilt"))
  (bind (_x _y) (Math|Vector2D|BreakVector2D ActionValue))
  (bind _sphere (Variables|Default|GetSphere))
  (:Triggered
    (Class|PrimitiveComponent|AddTorqueinRadians (Variables|Default|GetSphere) (Math|Conversions|ToVector(Vector2D) (* (Math|Vector2D|Normalize2D (Math|Vector2D|MakeVector2D (* _x -1.0) _y)) (Variables|Default|GetRollTorque))) "None" false))
  (:Started
    (Class|PrimitiveComponent|SetAngularDamping _sphere 0.0))
  (:Completed
    (Class|PrimitiveComponent|SetAngularDamping _sphere 5.0)))

(event EventBeginPlay
  (Input|AddMappingContext (PlayerController|LocalPlayerSubsystems|GetEnhancedInputLocalPlayerSubsystem (Game|GetPlayerController 0)) "/Game/Blueprints/Input/IMC_Default.IMC_Default" 0 "(bIgnoreAllPressedKeysUntilRelease=True,bForceImmediately=False,bNotifyUserSettings=False)")
  (Class|PrimitiveComponent|SetPhysicsMaxAngularVelocityinRadians (Variables|Default|GetSphere) (Variables|Default|GetMaxAngularVelocity) false "None")
  (bind _outactors (Actor|GetAllActorsOfClass "/Game/GoodSky/Blueprint/BP_GoodSky.BP_GoodSky_C"))
  (bind _array_element (Utilities|Array|ForEachLoopwithBreak _outactors :!label _label)
    (:LoopBody
      (Variables|Default|SetGoodSkyRef _array_element)
      (goto _label Break))))

(event EventTick
  (params (DeltaSeconds :type Float%20%28single-precision%29))
  (bind _returnvalue (Input|EnhancedActionValues|GetIA_Tilt))
  (bind _returnvalue_2 (Input|EnhancedActionValues|GetIA_Tilt))
  (bind _goodskyref (Variables|Default|GetGoodSkyRef))
  (bind _sphere (Variables|Default|GetSphere))
  (bind _springarm (Variables|Default|GetSpringArm))
  (bind _arrow (Variables|Default|GetArrow))
  (bind _springarm_2 (Variables|Default|GetSpringArm))
  (bind (_x _y) (Math|Vector2D|BreakVector2D _returnvalue))
  (bind (_x_2 _y_2) (Math|Vector2D|BreakVector2D _returnvalue_2))
  (bind _returnvalue_3 (Transformation|GetActorRotation _goodskyref))
  (bind _returnvalue_4 (Transformation|GetComponentVelocity _sphere))
  (bind _relativerotation (Variables|/Script/Engine.SceneComponent|GetRelativeRotation _springarm_2))
  (Utilities|FlowControl|Sequence
    (:then_0
      (Transformation|SetRelativeRotation _springarm_2 (Math|Rotator|Lerp(Rotator) _relativerotation (Math|Rotator|MakeRotator (* _x_2 -1.0 15.0) (* _y_2 1.0 1e+01) (.Yaw (Math|Rotator|BreakRotator _relativerotation))) (* (Utilities|Time|GetWorldDeltaSeconds) 5.0)) false false)
      (Variables|/Script/Engine.SpringArmComponent|SetTargetArmLength _springarm (Math|Float|Lerp (Variables|/Script/Engine.SpringArmComponent|GetTargetArmLength _springarm) (Math|Float|MapRangeClamped (Math|Vector|VectorLength (Transformation|GetComponentVelocity (Variables|Default|GetSphere))) 0.0 1.5e+03 5e+02 8e+02) (* (Utilities|Time|GetWorldDeltaSeconds) 5.0))))
    (:then_1
      (Transformation|SetActorRelativeRotation _goodskyref (Math|Rotator|Lerp(Rotator) _returnvalue_3 (Math|Rotator|MakeRotator (* _x -1.0 5.0) (* _y 1.0 8.0) (.Yaw (Math|Rotator|BreakRotator _returnvalue_3))) (* (Utilities|Time|GetWorldDeltaSeconds) 5.0))))
    (:then_2
      (Transformation|SetWorldRotation _arrow (Math|Rotator|MakeRotationfromAxes (Math|Vector|GetUnitDirection(Vector) (Variables|/Script/Engine.SceneComponent|GetRelativeLocation (Variables|Default|GetArrow)) _returnvalue_4) "0, 0, 0" "0, 0, 0") false false)
      (Variables|/Script/Engine.ArrowComponent|SetArrowLength _arrow (Math|Float|MapRangeClamped (Math|Vector|VectorLength _returnvalue_4) 0.0 1.5e+03 1.5e+02 3e+02)))))

(event Input|GamepadEvents|GamepadFaceButtonTop
  (params (Key :type Key%20Structure :default "None"))
  (bind _arrow (Variables|Default|GetArrow))
  (:Pressed
    (Development|SetHiddeninGame _arrow (not (Variables|/Script/Engine.SceneComponent|GetbHiddenInGame _arrow)) false)))

(event Input|KeyboardEvents|T
  (params (Key :type Key%20Structure :default "None"))
  (bind _arrow (Variables|Default|GetArrow))
  (:Pressed
    (Development|SetHiddeninGame _arrow (not (Variables|/Script/Engine.SceneComponent|GetbHiddenInGame _arrow)) false)))

(fn ConstructionScript)