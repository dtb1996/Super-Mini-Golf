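; Character Blueprint that changes its own gravity direction from keyboard input, apparently as a test of custom gravity.
; BeginPlay adds the default Enhanced Input mapping context, while the gravity switches use raw key events that set the direction on CharacterMovement.
; A flips gravity upward with no release handler; D pulls it along negative world X while held and restores downward gravity on release.
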(event EventBeginPlay
  (Input|AddMappingContext (PlayerController|LocalPlayerSubsystems|GetEnhancedInputLocalPlayerSubsystem (Game|GetPlayerController 0)) "/Game/Blueprints/Input/IMC_Default.IMC_Default" 0 "(bIgnoreAllPressedKeysUntilRelease=True,bForceImmediately=False,bNotifyUserSettings=False)"))

(event Collision|EventActorBeginOverlap
  (params (OtherActor :type Actor%20Object%20Reference)))

(event EventTick
  (params (DeltaSeconds :type Float%20%28single-precision%29)))

(event Input|KeyboardEvents|D
  (params (Key :type Key%20Structure :default "None"))
  (:Pressed
    (Class|CharacterMovementComponent|SetGravityDirection (Variables|Character|GetCharacterMovement) (Math|Vector|MakeVector -1.0 0.0 0.0)))
  (:Released
    (Class|CharacterMovementComponent|SetGravityDirection (Variables|Character|GetCharacterMovement) (Math|Vector|MakeVector 0.0 0.0 -1.0))))

(event Input|KeyboardEvents|A
  (params (Key :type Key%20Structure :default "None"))
  (:Pressed
    (Class|CharacterMovementComponent|SetGravityDirection (Variables|Character|GetCharacterMovement) (Math|Vector|MakeVector 0.0 0.0 1.0))))

(fn ConstructionScript)