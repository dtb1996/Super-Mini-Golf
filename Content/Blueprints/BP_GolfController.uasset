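; BP_GolfController is the golf game's controller, handling level-wide input and gating gameplay controls by game state.
; It subscribes to BP_GolfGameState changes, adding the default Enhanced Input mapping context when Active and removing it on Goal Reached or Failed.
; Input actions toggle pause, notifying BP_GolfGameInstance, and reload the current level.
; Raw keys set music volume through the game instance and quit the game.
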(event Custom|OnGameStateChanged
  (params (State :type EGameStates%20Enum :default "PreStart"))
  (switch Utilities|FlowControl|Switch|SwitchonEGameStates State
    (:Active
      (Input|AddMappingContext (PlayerController|LocalPlayerSubsystems|GetEnhancedInputLocalPlayerSubsystem self) "/Game/Blueprints/Input/IMC_Default.IMC_Default" 0 "(bIgnoreAllPressedKeysUntilRelease=True,bForceImmediately=False,bNotifyUserSettings=False)"))
    (:GoalReached
      (Input|RemoveMappingContext (PlayerController|LocalPlayerSubsystems|GetEnhancedInputLocalPlayerSubsystem self) "/Game/Blueprints/Input/IMC_Default.IMC_Default" "(bIgnoreAllPressedKeysUntilRelease=True,bForceImmediately=False,bNotifyUserSettings=False)" :!label _label))
    (:Failed
      (goto _label))))

(event Input|EnhancedActionEvents|EnhancedInputActionIA_Pause
  (params (ActionValue :type Boolean) (ElapsedSeconds :type Float%20%28double-precision%29) (TriggeredSeconds :type Float%20%28double-precision%29) (InputAction :type Input%20Action%20Object%20Reference :default "/Game/Blueprints/Input/Actions/IA_Pause.IA_Pause"))
  (Game|SetGamePaused (not (Game|IsGamePaused)))
  (bind _asbp_golf_game_instance (Utilities|Casting|CastToBP_GolfGameInstance (Game|GetGameInstance)))
  (Default|OnGamePausedChanged _asbp_golf_game_instance (Game|IsGamePaused)))

(event Input|EnhancedActionEvents|EnhancedInputActionIA_ResetLevel
  (params (ActionValue :type Boolean) (ElapsedSeconds :type Float%20%28double-precision%29) (TriggeredSeconds :type Float%20%28double-precision%29) (InputAction :type Input%20Action%20Object%20Reference :default "/Game/Blueprints/Input/Actions/IA_ResetLevel.IA_ResetLevel"))
  (bind _returnvalue (Game|GetCurrentLevelName true))
  (Game|OpenLevel(byName) (Utilities|String|StringToName _returnvalue)))

(event EventBeginPlay
  (bind _asbp_golf_game_state (Utilities|Casting|CastToBP_GolfGameState (Game|GetGameState)))
  (bind _output_get (Variables|Default|SetGameStateRef _asbp_golf_game_state))
  (EventDispatchers|BindEventtoStateChanged _output_get (EventDispatchers|CreateEvent :!event Custom|OnGameStateChanged)))

(event EventDestroyed
  (bind _gamestateref (Variables|Default|GetGameStateRef)
    (:then
      (EventDispatchers|UnbindEventfromStateChanged _gamestateref (EventDispatchers|CreateEvent :!event Custom|OnGameStateChanged)))
    (:else)))

(event Input|KeyboardEvents|M
  (params (Key :type Key%20Structure :default "None"))
  (:Pressed
    (bind _asbp_golf_game_instance (Utilities|Casting|CastToBP_GolfGameInstance (Game|GetGameInstance)))
    (Default|SetMusicVolume _asbp_golf_game_instance 1.0)))

(event Input|KeyboardEvents|Escape
  (params (Key :type Key%20Structure :default "None"))
  (:Pressed
    (Game|QuitGame 0 "Quit" false)))

(fn ConstructionScript)