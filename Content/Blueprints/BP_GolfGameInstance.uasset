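; Game instance for the golf game that owns background music playback across level transitions.
; PlayAudioTrack spawns a persistent 2D sound, stores it as CurrentAudioTrack and drops it to near-silence until a volume setting is connected.
; SetMusicVolume and IsPlayingMusic act on that stored component after a validity check.
; StopAudioPlayback clears the reference before calling Stop on it, so the Stop call targets an empty reference.
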(event Custom|PlayAudioTrack
  (params (Track :type Sound%20Base%20Object%20Reference))
  (bind _returnvalue (Audio|SpawnSound2D Track 1.0 1.0 0.0 0 true false))
  (bind _output_get (Variables|Default|SetCurrentAudioTrack _returnvalue))
  ;[1 1 1] TODO: remove and connect to volume setting
  (Audio|Components|Audio|AdjustVolume _output_get 0.0 1e-05 "Linear" :!class /Script/Engine.AudioComponent))

(event Custom|StopAudioPlayback
  (bind _output_get (Variables|Default|SetCurrentAudioTrack 0))
  (Audio|Components|Audio|Stop _output_get))

(event Custom|SetMusicVolume
  (params (NewVolume :type Float%20%28single-precision%29))
  (bind _currentaudiotrack (Variables|Default|GetCurrentAudioTrack)
    (:then
      (Audio|Components|Audio|AdjustVolume _currentaudiotrack 0.0 NewVolume "Linear" :!class /Script/Engine.AudioComponent))
    (:else)))

(fn IsPlayingMusic
  (bind _currentaudiotrack (Variables|Default|GetCurrentAudioTrack)
    (:then
      (return (Audio|Components|Audio|IsPlaying _currentaudiotrack)))
    (:else
      (return false))))