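; Game state for a golf game that tracks each attempt's phase, from countdown and active play through goal reached or failed to results and level change.
; Phase events set ActiveState and broadcast it; countdown and attempt timers fire their own dispatchers on expiry.
; BeginPlay caches the level's time limit and collectible count.
; GetAttemptResults scores clear and all-collectible bonuses into a map and updates the player's score.
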(event Custom|RunPreAttemptStateLogic
  (params (TimeLength :type Float%20%28double-precision%29))
  (bind _output_get (Variables|Default|SetActiveState "Countdown"))
  (Default|CallStateChanged _output_get)
  (bind _returnvalue (Utilities|Time|SetTimerbyFunctionName 0 "PreStartTimerEnded" TimeLength))
  (Variables|Default|SetPreAttemptTimer _returnvalue))

(event Custom|RunStartAttemptLogic
  (params (AttemptTimeLength :type Float%20%28double-precision%29))
  (bind _output_get (Variables|Default|SetActiveState "Active"))
  (Default|CallStateChanged _output_get)
  (bind _returnvalue (Utilities|Time|SetTimerbyFunctionName 0 "AttemptTimerEnded" (Variables|Default|GetAttemptTimeLength)))
  (Variables|Default|SetAttemptTimer _returnvalue))

(event Custom|RunFailedAttemptLogic
  (bind _output_get (Variables|Default|SetActiveState "Failed"))
  (Default|CallStateChanged _output_get))

(event Custom|RunGoalReachedLogic
  (bind _output_get (Variables|Default|SetActiveState "GoalReached"))
  (Default|CallStateChanged _output_get))

(event Custom|RunChangingLevelLogic
  (bind _output_get (Variables|Default|SetActiveState "ChangingLevel"))
  (Default|CallStateChanged _output_get))

(event Custom|PreStartTimerEnded
  (Default|CallPreStartTimerTriggered))

(event Custom|AttemptTimerEnded
  (Default|CallAttemptTimerTriggered))

(event Custom|DisplayResults
  (bind _output_get (Variables|Default|SetActiveState "ResultsScreen"))
  (Default|CallStateChanged _output_get)
  (Class|UILayersManagerFunctionLibrary|PushContenttoLayer (Game|GetPlayerController 0) "(TagName=\"UI.Layer.GameMenu\")" "/Game/Blueprints/UI/Game/WBP_ResultsScreen.WBP_ResultsScreen_C"))

(event EventBeginPlay
  (Utilities|FlowControl|Sequence
    (:then_0
      (bind _asbp_golf_game_instance (Utilities|Casting|CastToBP_GolfGameInstance (Game|GetGameInstance)))
      (Variables|Default|SetAttemptTimeLength (Utilities|Struct|BreakS_LevelDetails (Default|GetCurrentLevelInfo _asbp_golf_game_instance))))
    (:then_1
      (bind _outactors (Actor|GetAllActorsOfClass "/Game/Blueprints/GameLogic/BP_Collectible.BP_Collectible_C"))
      (Variables|Default|SetTotalCollectibles (Utilities|Array|Length _outactors)))))

(fn ConstructionScript)

(fn GetAttemptRemainingTime
  (return (Utilities|Time|GetTimerRemainingTimebyHandle (Variables|Default|GetAttemptTimer))))

(fn GetAttemptTimeLength
  (return (Variables|Default|GetAttemptTimeLength)))

(fn GetTotalCollectiblesinLevel
  (return (Variables|Default|GetTotalCollectibles)))

(fn GetAttemptResults
  (bind _asbp_golf_player_state (Utilities|Casting|CastToBP_GolfPlayerState (Game|GetPlayerState 0))
    (:then
      (LocalVariables|SetPlayerStateRef _asbp_golf_player_state)
      (bind _enumvalue (|ForEachE_ResultsConditionsToCheck)
        (:LoopBody
          (switch Utilities|FlowControl|Switch|SwitchonE_ResultsConditionsToCheck _enumvalue
            (:NewEnumerator0
              (Utilities|Map|Add (LocalVariables|GetResultsMap) "Stage Clear" 100)
              (LocalVariables|SetPointsEarned (+ (LocalVariables|GetPointsEarned) 100)))
            (:NewEnumerator1
              (bind _playerstateref (LocalVariables|GetPlayerStateRef)
                (:then
                  (if (>= (.CurrentCoins (Utilities|Struct|BreakPlayerStats (Default|GetPlayerStats _playerstateref))) (CallFunction|GetTotalCollectiblesinLevel))
                    (Utilities|Map|Add (LocalVariables|GetResultsMap) "All Collectibles" 200)
                    (LocalVariables|SetPointsEarned (+ (LocalVariables|GetPointsEarned) 200))))
                (:else)))))
        (:then
          (Utilities|FlowControl|Sequence
            (:then_0
              (Utilities|Map|Add (LocalVariables|GetResultsMap) "Points" (LocalVariables|GetPointsEarned))
              (bind _playerstateref_2 (LocalVariables|GetPlayerStateRef)
                (:then
                  (Default|AddtoPlayerScore _playerstateref_2 (LocalVariables|GetPointsEarned)))
                (:else)))
            (:then_1
              (bind _playerstateref_3 (LocalVariables|GetPlayerStateRef)
                (:then
                  (Utilities|Map|Add (LocalVariables|GetResultsMap) "Total Points" (Utilities|Struct|BreakPlayerStats (Default|GetPlayerStats _playerstateref_3))))
                (:else)))
            (:then_2
              (return (LocalVariables|GetResultsMap)))))))
    (:CastFailed
      (Development|PrintString "BP_GolfGameState - ERROR: BP_GolfPlayerState cast failed"))))