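; Golf ball pawn that exposes tuning for rolling, tilting and hit impulse, and takes physics impulses on its collision sphere.
; On BeginPlay it attaches the first BP_GoodSky actor to its SpringArm, keeping world location and scale and relative rotation.
; Getter and setter functions expose the movement settings, while CollectCoins forwards coin pickups to the player state.
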(event EventBeginPlay
  (|CallParentFunction)
  (bind _outactors (Actor|GetAllActorsOfClass "/Game/GoodSky/Blueprint/BP_GoodSky.BP_GoodSky_C"))
  (bind _array_element (Utilities|Array|ForEachLoopwithBreak _outactors :!label _label)
    (:LoopBody
      (bind _output_get (Variables|Default|SetSkySphere _array_element))
      (Transformation|AttachComponentToComponent _output_get (Variables|Default|GetSpringArm) "None" "KeepWorld" "KeepRelative" "KeepWorld" true)
      (goto _label Break))))

(fn ConstructionScript)

(fn GetPawnSettings
  (return (Variables|Default|GetRollTorque) (Variables|Default|GetTiltAngularDamping) (Variables|Default|GetNormalAngularDamping) (Variables|Default|GetMaxAngularVelocity) (Variables|Default|GetTiltFactorX) (Variables|Default|GetTiltFactorY) (Variables|Default|GetHitImpulseMin)))

(fn SetRollTorque
  (params (RollTorque :type Float%20%28single-precision%29))
  (Variables|Default|SetRollTorque RollTorque))

(fn SetTiltAngularDamping
  (params (TiltAngularDamping :type Float%20%28single-precision%29))
  (Variables|Default|SetTiltAngularDamping TiltAngularDamping))

(fn SetNormalAngularDamping
  (params (NormalAngularDamping :type Float%20%28single-precision%29))
  (Variables|Default|SetNormalAngularDamping NormalAngularDamping))

(fn SetMaxAngularVelocity
  (params (MaxAngularVelocity :type Float%20%28single-precision%29))
  (Variables|Default|SetMaxAngularVelocity MaxAngularVelocity))

(fn SetTiltFactorX
  (params (TiltFactorX :type Float%20%28single-precision%29))
  (Variables|Default|SetTiltFactorX TiltFactorX))

(fn SetTiltFactorY
  (params (TiltFactorY :type Float%20%28single-precision%29))
  (Variables|Default|SetTiltFactorY TiltFactorY))

(fn SetHitImpulseMin
  (params (HitImpulseMin :type Float%20%28single-precision%29))
  (Variables|Default|SetHitImpulseMin HitImpulseMin))

(fn ApplyImpulse
  (params (Impulse :type Vector :default "0, 0, 0"))
  (Physics|AddImpulse (Variables|Default|GetSphereCollision) Impulse "None" false)
  (return true))

(fn CollectCoins
  (params (NumCoins :type Integer))
  (bind _success (Class|IInteract|CollectCoins(Message) (Game|GetPlayerState 0) NumCoins))
  (return _success))