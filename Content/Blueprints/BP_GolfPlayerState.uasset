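; Player state for a golf game that tracks the player's coin count and score.
; CollectCoins adds the given coins, raises the score by a flat 50 regardless of amount, and returns true.
; Both setters fire update dispatchers with the new value; SetCurrentCoins adds to the running total rather than replacing it, while SetPlayerScore overwrites.
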(event EventBeginPlay)

(fn ConstructionScript)

(fn GetCurrentCoins
  (return (Variables|Default|GetCurrentCoins)))

(fn SetCurrentCoins
  (params (InputPin :type Integer))
  (bind _output_get (Variables|Default|SetCurrentCoins (+ InputPin (Variables|Default|GetCurrentCoins))))
  (Default|CallCoinCountUpdated _output_get))

(fn SetPlayerScore
  (params (NewPlayerScore :type Integer))
  (bind _output_get (Variables|Default|SetPlayerScore NewPlayerScore))
  (Default|CallPlayerScoreUpdated _output_get))

(fn GetPlayerScore
  (return (Variables|Default|GetPlayerScore)))

(fn CollectCoins
  (params (NumCoins :type Integer))
  (CallFunction|SetCurrentCoins NumCoins)
  (CallFunction|SetPlayerScore (+ (CallFunction|GetPlayerScore) 50))
  (return true))