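; BP_Conveyor is a conveyor belt actor that moves any actor inside its Box along the static mesh's forward direction.
; Each tick it offsets every overlapping actor by Speed scaled by delta time, without sweeping for collisions.
; The construction script applies a dynamic M_Conveyor material instance to the mesh, setting its color and the arrow scale and speed from variables independent of the push speed.
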(event EventTick
  (params (DeltaSeconds :type Float%20%28single-precision%29))
  (for _array_element (Collision|GetOverlappingActors (Variables|Default|GetBox) 0 :!class /Script/Engine.PrimitiveComponent)
    (Transformation|AddActorWorldOffset _array_element (* (Math|Vector|GetForwardVector (Transformation|GetWorldRotation (Variables|Default|GetStaticMesh))) (* (Utilities|Time|GetWorldDeltaSeconds) (Variables|Default|GetSpeed))))))

(fn ConstructionScript
  (bind _returnvalue (Rendering|Material|CreateDynamicMaterialInstance (Variables|Default|GetStaticMesh) 0 "/Game/Materials/M_Conveyor.M_Conveyor" "None" :!class /Script/Engine.PrimitiveComponent))
  (Rendering|Material|SetMaterial (Variables|Default|GetStaticMesh) 0 _returnvalue)
  (Rendering|Material|SetVectorParameterValue _returnvalue "Color" (Variables|Default|GetColor) :!class /Script/Engine.MaterialInstanceDynamic)
  (Rendering|Material|SetScalarParameterValue _returnvalue "XScale" (Variables|Default|GetArrowScale) :!class /Script/Engine.MaterialInstanceDynamic)
  (Rendering|Material|SetScalarParameterValue _returnvalue "XSpeed" (Variables|Default|GetArrowSpeed) :!class /Script/Engine.MaterialInstanceDynamic))