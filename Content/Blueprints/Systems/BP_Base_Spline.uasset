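; Base spline actor that builds a chain of spline meshes along its spline in the construction script.
; Each section spans SectionLength, which AllowScaling derives from actor scale on the mesh's forward axis.
; Helper functions supply local-space endpoints, with tangents clamped to section length to fit each segment.
; Mesh, forward axis and collision type are configurable, and MustBeFullLengthMeshes drops the shorter final piece.
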(event EventBeginPlay)

(event Collision|EventActorBeginOverlap
  (params (OtherActor :type Actor%20Object%20Reference)))

(event EventTick
  (params (DeltaSeconds :type Float%20%28single-precision%29)))

(fn ConstructionScript
  (bind _returnvalue (Transformation|GetActorScale3D))
  (bind (_x _y _z) (Math|Vector|BreakVector _returnvalue))
  (if (Variables|Default|GetbAllowScaling)
    (Variables|Default|SetSectionLength (* (Utilities|Select :Index (Variables|Default|GetMeshForwardAxis) :X _x :Y _y :Z _z) 1e+02)))
  (for _index (range 0 (select (Variables|Default|GetbMustBeFullLengthMeshes) (- (Math|Float|Truncate (/ (Spline|GetSplineLength (Variables|Default|GetSpline)) (Variables|Default|GetSectionLength))) 1) (Math|Float|Truncate (/ (Spline|GetSplineLength (Variables|Default|GetSpline)) (Variables|Default|GetSectionLength)))))
    (LocalVariables|SetLOCAL_LoopIndex _index)
    (bind _returnvalue_2 (AddComponent|AddSplineMeshComponent false))
    (Components|StaticMesh|SetStaticMesh _returnvalue_2 (Variables|Default|GetSplineMesh))
    (SplineMesh|SetForwardAxis _returnvalue_2 (Variables|Default|GetMeshForwardAxis) true)
    (SplineMesh|SetStartandEnd _returnvalue_2 (.Position (CallFunction|GetStartPositionandTangent (LocalVariables|GetLOCAL_LoopIndex))) (.Tangent (CallFunction|GetStartPositionandTangent (LocalVariables|GetLOCAL_LoopIndex))) (.Position (CallFunction|GetEndPositionandTangent (LocalVariables|GetLOCAL_LoopIndex))) (.Tangent (CallFunction|GetEndPositionandTangent (LocalVariables|GetLOCAL_LoopIndex))) true :!class /Script/Engine.SplineMeshComponent)
    (Collision|SetCollisionEnabled _returnvalue_2 (Variables|Default|GetCollisionType))))

(fn GetStartPositionandTangent
  (params (Index :type Integer))
  (bind _spline (Variables|Default|GetSpline))
  (bind _sectionlength (Variables|Default|GetSectionLength))
  (bind _returnvalue (* Index _sectionlength))
  (return (Spline|GetLocationatDistanceAlongSpline _spline _returnvalue "Local") (Math|Vector|ClampVectorSize (Spline|GetTangentatDistanceAlongSpline _spline _returnvalue "Local") 0.0 (Variables|Default|GetSectionLength))))

(fn GetEndPositionandTangent
  (params (Index :type Integer))
  (bind _spline (Variables|Default|GetSpline))
  (bind _sectionlength (Variables|Default|GetSectionLength))
  (bind _returnvalue (+ Index 1))
  (bind _returnvalue_2 (* _returnvalue _sectionlength))
  (return (Spline|GetLocationatDistanceAlongSpline _spline _returnvalue_2 "Local") (Math|Vector|ClampVectorSize (Spline|GetTangentatDistanceAlongSpline _spline _returnvalue_2 "Local") 0.0 (Variables|Default|GetSectionLength))))