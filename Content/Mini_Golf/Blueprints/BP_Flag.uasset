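; BP_Flag is the mini-golf hole flag, which reacts to a nearby GolfPawn and detects when the goal is reached.
; The near sphere plays and reverses a timeline driving the flag's scale and height.
; The hole sphere uses a DoOnce to notify BP_GolfGameMode a single time.
; The construction script picks the flag mesh from an enum-keyed map, with one option hiding the flag and disabling near-sphere collision.
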(event OnComponentBeginOverlap(Sphere_Near)
  (params (OverlappedComponent :type Primitive%20Component%20Object%20Reference) (OtherActor :type Actor%20Object%20Reference) (OtherComp :type Primitive%20Component%20Object%20Reference) (OtherBodyIndex :type Integer) (bFromSweep :type Boolean) (SweepResult :type Hit%20Result%20Structure%20%28by%20ref%29))
  (if (Class|GameplayStatics|ObjectIsA OtherActor "/Script/SuperMiniGolf.GolfPawn")
    (bind (_direction _scale _z_position) (Timeline|Timeline_FlagScale Play)
      (:Update
        (Transformation|SetRelativeScale3D (Variables|Default|GetFlagSkeletalMesh) _scale)
        (Transformation|SetRelativeLocation (Variables|Default|GetFlagSkeletalMesh) (Math|Vector|MakeVector 0.0 0.0 _z_position) false false)))))

(event OnComponentEndOverlap(Sphere_Near)
  (params (OverlappedComponent :type Primitive%20Component%20Object%20Reference) (OtherActor :type Actor%20Object%20Reference) (OtherComp :type Primitive%20Component%20Object%20Reference) (OtherBodyIndex :type Integer))
  (if (Class|GameplayStatics|ObjectIsA OtherActor "/Script/SuperMiniGolf.GolfPawn")
    (bind (_direction _scale _z_position) (Timeline|Timeline_FlagScale Reverse)
      (:Update
        (Transformation|SetRelativeScale3D (Variables|Default|GetFlagSkeletalMesh) _scale)
        (Transformation|SetRelativeLocation (Variables|Default|GetFlagSkeletalMesh) (Math|Vector|MakeVector 0.0 0.0 _z_position) false false)))))

(event OnComponentBeginOverlap(Sphere_Hole)
  (params (OverlappedComponent :type Primitive%20Component%20Object%20Reference) (OtherActor :type Actor%20Object%20Reference) (OtherComp :type Primitive%20Component%20Object%20Reference) (OtherBodyIndex :type Integer) (bFromSweep :type Boolean) (SweepResult :type Hit%20Result%20Structure%20%28by%20ref%29))
  (if (Class|GameplayStatics|ObjectIsA OtherActor "/Script/SuperMiniGolf.GolfPawn")
    (Utilities|FlowControl|DoOnce false
      (:Completed
        (bind _asbp_golf_game_mode (Utilities|Casting|CastToBP_GolfGameMode (Game|GetGameMode)))
        (Default|PlayerGoalReached _asbp_golf_game_mode)))))

(fn ConstructionScript
  (if (not (Utilities|Enum|Equal(Enum) (Variables|Default|GetFlagMesh) "NewEnumerator2"))
    (Components|SkeletalMesh|SetSkeletalMeshAsset (Variables|Default|GetFlagSkeletalMesh) (.Value (Utilities|Map|Find (LocalVariables|GetFlagMeshMap) (Variables|Default|GetFlagMesh))))
    (else
      (Rendering|SetVisibility (Variables|Default|GetFlagSkeletalMesh) false false)
      (Collision|SetCollisionEnabled (Variables|Default|GetSphere_Near) "NoCollision"))))