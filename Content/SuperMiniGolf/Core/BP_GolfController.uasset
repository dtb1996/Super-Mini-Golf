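; Player controller for the mini golf game that handles pausing, level restart and gameplay input availability.
; It binds to game state changes, enabling the default Enhanced Input context when Active and removing it on goal or failure.
; Pausing pushes a UI layer menu, notifies the game instance and toggles the menu input context.
; Hard-coded debug keys open pawn settings, toggle the layout debugger and near-mute music.
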(event Custom|OnGameStateChanged
  (params (State :type EGameStates%20Enum :default "PreStart"))
  (switch Utilities|FlowControl|Switch|SwitchonEGameStates State
    (:Active
      (Input|AddMappingContext (PlayerController|LocalPlayerSubsystems|GetEnhancedInputLocalPlayerSubsystem self) "/Game/SuperMiniGolf/Core/Input/IMC_Default.IMC_Default" 0 "(bIgnoreAllPressedKeysUntilRelease=True,bForceImmediately=False,bNotifyUserSettings=False)"))
    (:GoalReached
      (Input|RemoveMappingContext (PlayerController|LocalPlayerSubsystems|GetEnhancedInputLocalPlayerSubsystem self) "/Game/SuperMiniGolf/Core/Input/IMC_Default.IMC_Default" "(bIgnoreAllPressedKeysUntilRelease=True,bForceImmediately=False,bNotifyUserSettings=False)" :!label _label))
    (:Failed
      (goto _label))
    (:ResultsScreen
      (Variables|Default|SetbShowMouseCursor false))))

(event Custom|Unpause
  (bind _returnvalue (Game|IsGamePaused))
  (Variables|/Script/Engine.PlayerController|SetbShowMouseCursor self false)
  (Game|SetGamePaused false)
  (bind _asbp_golf_game_instance (Utilities|Casting|CastToBP_GolfGameInstance (Game|GetGameInstance))
    (:then
      (Default|OnGamePausedChanged _asbp_golf_game_instance _returnvalue))
    (:CastFailed
      _))
  (if _returnvalue
    (Input|AddMappingContext (PlayerController|LocalPlayerSubsystems|GetEnhancedInputLocalPlayerSubsystem self) "/Game/SuperMiniGolf/Core/Input/IMC_Menu.IMC_Menu" 0 "(bIgnoreAllPressedKeysUntilRelease=True,bForceImmediately=False,bNotifyUserSettings=False)")
    (else
      (Input|RemoveMappingContext (PlayerController|LocalPlayerSubsystems|GetEnhancedInputLocalPlayerSubsystem self) "/Game/SuperMiniGolf/Core/Input/IMC_Menu.IMC_Menu" "(bIgnoreAllPressedKeysUntilRelease=True,bForceImmediately=False,bNotifyUserSettings=False)"))))

(event Input|EnhancedActionEvents|EnhancedInputActionIA_Pause
  (params (ActionValue :type Boolean) (ElapsedSeconds :type Float%20%28double-precision%29) (TriggeredSeconds :type Float%20%28double-precision%29) (InputAction :type Input%20Action%20Object%20Reference :default "/Game/SuperMiniGolf/Core/Input/Actions/IA_Pause.IA_Pause"))
  (bind _returnvalue (Game|IsGamePaused))
  (bind _returnvalue_2 (Game|IsGamePaused))
  (bind _returnvalue_3 (not _returnvalue_2))
  (if _returnvalue_3
    (Class|UILayersManagerFunctionLibrary|PushContenttoLayer self "(TagName=\"UI.Layer.Menu\")" "/Game/SuperMiniGolf/UI/GameMenu/WBP_PauseMenu.WBP_PauseMenu_C")
    (Variables|/Script/Engine.PlayerController|SetbShowMouseCursor self true)
    (Game|SetGamePaused _returnvalue_3)
    (bind _asbp_golf_game_instance (Utilities|Casting|CastToBP_GolfGameInstance (Game|GetGameInstance))
      (:then
        (Default|OnGamePausedChanged _asbp_golf_game_instance _returnvalue))
      (:CastFailed
        _))
    (if _returnvalue
      (Input|AddMappingContext (PlayerController|LocalPlayerSubsystems|GetEnhancedInputLocalPlayerSubsystem self) "/Game/SuperMiniGolf/Core/Input/IMC_Menu.IMC_Menu" 0 "(bIgnoreAllPressedKeysUntilRelease=True,bForceImmediately=False,bNotifyUserSettings=False)")
      (else
        (Input|RemoveMappingContext (PlayerController|LocalPlayerSubsystems|GetEnhancedInputLocalPlayerSubsystem self) "/Game/SuperMiniGolf/Core/Input/IMC_Menu.IMC_Menu" "(bIgnoreAllPressedKeysUntilRelease=True,bForceImmediately=False,bNotifyUserSettings=False)")))))

(event Input|EnhancedActionEvents|EnhancedInputActionIA_ResetLevel
  (params (ActionValue :type Boolean) (ElapsedSeconds :type Float%20%28double-precision%29) (TriggeredSeconds :type Float%20%28double-precision%29) (InputAction :type Input%20Action%20Object%20Reference :default "/Game/SuperMiniGolf/Core/Input/Actions/IA_ResetLevel.IA_ResetLevel"))
  (bind _returnvalue (Game|GetCurrentLevelName true))
  (Game|OpenLevel(byName) (Utilities|String|StringToName _returnvalue)))

(event EventBeginPlay
  (bind _asbp_golf_game_state (Utilities|Casting|CastToBP_GolfGameState (Game|GetGameState)))
  (bind _output_get (Variables|Default|SetGameStateRef _asbp_golf_game_state))
  (EventDispatchers|BindEventtoStateChanged _output_get (EventDispatchers|CreateEvent :!event Custom|OnGameStateChanged)))

(event EventDestroyed
  (bind _gamestateref (Variables|Default|GetGameStateRef)
    (:then
      (EventDispatchers|UnbindEventfromStateChanged _gamestateref (EventDispatchers|CreateEvent :!event Custom|OnGameStateChanged)))
    (:else)))

(event Input|KeyboardEvents|Shift2
  (params (Key :type Key%20Structure))
  (:Pressed
    (bind _foundwidgets (Widget|GetAllWidgetsOfClass "/UILayersManager/WBP_PrimaryLayout.WBP_PrimaryLayout_C" true))
    (Default|CloseLayersDebugger (Utilities|Array|Get(acopy) _foundwidgets))))

(event Input|KeyboardEvents|1
  (params (Key :type Key%20Structure))
  (:Pressed
    (Class|UILayersManagerFunctionLibrary|PushContenttoLayer self "(TagName=\"UI.Layer.Debug\")" "/Game/SuperMiniGolf/UI/Debug/WBP_PlayerPawnSettings.WBP_PlayerPawnSettings_C")
    (Variables|/Script/Engine.PlayerController|SetbShowMouseCursor self true)
    (Input|SetInputModeGameandUI self 0 "DoNotLock" false true)))

(event Input|KeyboardEvents|M
  (params (Key :type Key%20Structure))
  (:Pressed
    (bind _asbp_golf_game_instance (Utilities|Casting|CastToBP_GolfGameInstance (Game|GetGameInstance)))
    (Default|SetMusicVolume _asbp_golf_game_instance 0.0001)))

(event Input|KeyboardEvents|2
  (params (Key :type Key%20Structure))
  (:Pressed
    (bind _foundwidgets (Widget|GetAllWidgetsOfClass "/UILayersManager/WBP_PrimaryLayout.WBP_PrimaryLayout_C" true))
    (Default|OpenLayersDebugger (Utilities|Array|Get(acopy) _foundwidgets))))

(fn ConstructionScript)