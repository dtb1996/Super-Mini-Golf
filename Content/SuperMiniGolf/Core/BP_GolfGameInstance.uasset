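; Game instance for SuperMiniGolf that keeps music and course progression across level loads.
; It plays one persistent 2D music track at a time, skipping restarts of the same track, with volume control and a low-pass muffle while paused.
; SetLevels queues row names from the level details data table; GetNextLevel pops the first and caches its row as the current level info.
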(event Custom|StopAudioPlayback
  (bind _currentaudiotrack (Variables|Default|GetCurrentAudioTrack)
    (:then
      (Audio|Components|Audio|Stop _currentaudiotrack)
      (Variables|Default|SetCurrentAudioTrack 0))
    (:else)))

(event Custom|SetMusicVolume
  (params (NewVolume :type Float%20%28single-precision%29))
  (bind _currentaudiotrack (Variables|Default|GetCurrentAudioTrack)
    (:then
      (Audio|Components|Audio|AdjustVolume _currentaudiotrack 0.0 NewVolume "Linear" :!class /Script/Engine.AudioComponent))
    (:else)))

(event Custom|OnGamePausedChanged
  (params (NewPaused :type Boolean))
  (bind _currentaudiotrack (Variables|Default|GetCurrentAudioTrack)
    (:then
      (Audio|Components|Audio|SetLowPassFilterEnabled _currentaudiotrack NewPaused :!class /Script/Engine.AudioComponent)
      (Audio|Components|Audio|SetLowPassFilterFrequency _currentaudiotrack (select NewPaused 2.5e+02 0.0) :!class /Script/Engine.AudioComponent))
    (:else)))

(event Custom|PlayAudioTrack
  (params (Track :type Sound%20Base%20Object%20Reference))
  (bind _currentaudiotrack (Variables|Default|GetCurrentAudioTrack)
    (:then
      (if (not (== (Variables|/Script/Engine.AudioComponent|GetSound _currentaudiotrack) Track))
        (CallFunction|StopAudioPlayback)
        (bind _returnvalue (Audio|SpawnSound2D Track 1.0 1.0 0.0 0 true false :!label _label))
        (bind _output_get (Variables|Default|SetCurrentAudioTrack _returnvalue))))
    (:else
      (goto _label))))

(event Custom|SetLevels
  (params (CourseDataTable :type Data%20Table%20Object%20Reference))
  (bind _output_get (Variables|Default|SetCourseDataTable "/Game/SuperMiniGolf/Core/Data/DT_LevelDetails.DT_LevelDetails"))
  (bind _outrownames (DataTable|GetDataTableRowNames _output_get))
  (Variables|Default|SetLevelQueue _outrownames))

(fn IsPlayingMusic
  (bind _currentaudiotrack (Variables|Default|GetCurrentAudioTrack)
    (:then
      (return (Audio|Components|Audio|IsPlaying _currentaudiotrack)))
    (:else
      (return false))))

(fn GetNextLevel
  (if (== (Variables|Default|GetCourseDataTable) "/Game/SuperMiniGolf/Core/Data/DT_LevelDetails.DT_LevelDetails")
    (bind _returnvalue (Utilities|GetDataTableRow "/Game/SuperMiniGolf/Core/Data/DT_LevelDetails.DT_LevelDetails" (Utilities|Array|Get(acopy) (Variables|Default|GetLevelQueue)))
      (:then
        (Utilities|Array|RemoveIndex (Variables|Default|GetLevelQueue))
        (bind _output_get (Variables|Default|SetCurrentLevel _returnvalue))
        (return _output_get)))))

(fn GetCurrentLevelInfo
  (return (Variables|Default|GetCurrentLevel)))