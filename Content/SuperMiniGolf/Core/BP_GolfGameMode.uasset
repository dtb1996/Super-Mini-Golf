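; Game mode for Super Mini Golf that runs the attempt flow on a level and handles the move to the next one.
; It forwards goal, fall-off, timer and next-level events to BP_GolfGameState, then reacts to its state changes.
; Countdown spawns and possesses a pawn, failure retries, and a goal advances the player index or shows results after the last player.
; Level info and music playback come from BP_GolfGameInstance.
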(event Custom|OnGameStateChanged
  (params (State :type EGameStates%20Enum :default "PreStart"))
  (Development|PrintString (Utilities|String|EnumtoString State))
  (switch Utilities|FlowControl|Switch|SwitchonEGameStates State
    (:Countdown
      (bind _outactors (Actor|GetAllActorsOfClass "/Script/Engine.PlayerStart"))
      (bind _returnvalue (Game|SpawnActorfromClass "/Game/SuperMiniGolf/Core/BP_GolfPawn.BP_GolfPawn_C" (Transformation|GetActorTransform (Utilities|Array|Get(acopy) _outactors)) "Undefined" "MultiplyWithRoot" 0 0))
      (Pawn|Possess (Game|GetPlayerController 0) _returnvalue))
    (:GoalReached
      (if (>= (Variables|Default|GetCurrentPlayerId) (- (Variables|Default|GetNumPlayers) 1))
        (Class|UILayersManagerFunctionLibrary|ClearLayer (Game|GetPlayerController 0) "(TagName=\"UI.Layer.Game\")")
        (bind _gamestateref (Variables|Default|GetGameStateRef)
          (:then
            (Default|DisplayResults _gamestateref))
          (:else))
        (else
          (Math|Integer|IncrementInt (Variables|Default|GetCurrentPlayerId)
            (:%20%20
              (bind _gamestateref_2 (Variables|Default|GetGameStateRef)
                (:then
                  (Default|RunPreAttemptStateLogic _gamestateref_2 2.0))
                (:else)))))))
    (:Failed
      (Actor|DestroyActor (Pawn|GetControlledPawn (Game|GetPlayerController 0)))
      (bind _gamestateref_3 (Variables|Default|GetGameStateRef)
        (:then
          (Default|RunPreAttemptStateLogic _gamestateref_3 2.0))
        (:else)))
    (:ChangingLevel
      (bind _gameinstanceref (Variables|Default|GetGameInstanceRef)
        (:then
          (bind _output_get (Variables|Default|SetCurrentLevelInfo (Default|GetNextLevel _gameinstanceref)))
          (Game|OpenLevel(byObjectReference) (Utilities|Struct|BreakSoftWorldReference (Utilities|Struct|BreakS_LevelDetails _output_get))))
        (:else)))))

(event Custom|PlayerGoalReached
  (params (PlayerId :type Integer))
  (bind _gamestateref (Variables|Default|GetGameStateRef)
    (:then
      (Default|RunGoalReachedLogic _gamestateref))
    (:else)))

(event Custom|OnPreGameTimerTriggered
  (bind _gamestateref (Variables|Default|GetGameStateRef)
    (:then
      (Default|RunStartAttemptLogic _gamestateref 6e+01))
    (:else)))

(event Custom|PlayerFallOff
  (bind _gamestateref (Variables|Default|GetGameStateRef)
    (:then
      (Default|RunFailedAttemptLogic _gamestateref))
    (:else)))

(event Custom|RequestNextLevel
  (bind _gamestateref (Variables|Default|GetGameStateRef)
    (:then
      (Default|RunChangingLevelLogic _gamestateref))
    (:else)))

(event EventPostLogin
  (params (NewPlayer :type Player%20Controller%20Object%20Reference))
  (Development|PrintString (Utilities|String|Append (Utilities|GetDisplayName NewPlayer) " - Login")))

(event EventDestroyed
  (bind _gamestateref (Variables|Default|GetGameStateRef)
    (:then
      (EventDispatchers|UnbindEventfromStateChanged _gamestateref (EventDispatchers|CreateEvent :!event Custom|OnGameStateChanged))
      (EventDispatchers|UnbindEventfromPreStartTimerTriggered _gamestateref (EventDispatchers|CreateEvent :!event Custom|OnPreGameTimerTriggered)))
    (:else)))

(event EventBeginPlay
  (Utilities|FlowControl|Sequence
    (:then_0
      (bind _asbp_golf_game_instance (Utilities|Casting|CastToBP_GolfGameInstance (Game|GetGameInstance)))
      (bind _output_get (Variables|Default|SetGameInstanceRef _asbp_golf_game_instance))
      (Variables|Default|SetCurrentLevelInfo (Default|GetCurrentLevelInfo _output_get))
      (Default|PlayAudioTrack (Variables|Default|GetGameInstanceRef) "/Game/SuperMiniGolf/Music/Andy_Youngman_-_Never_ever.Andy_Youngman_-_Never_ever"))
    (:then_1
      (bind _asbp_golf_game_state (Utilities|Casting|CastToBP_GolfGameState (Game|GetGameState)))
      (bind _output_get_2 (Variables|Default|SetGameStateRef _asbp_golf_game_state))
      (EventDispatchers|BindEventtoStateChanged _output_get_2 (EventDispatchers|CreateEvent :!event Custom|OnGameStateChanged))
      (EventDispatchers|BindEventtoPreStartTimerTriggered _output_get_2 (EventDispatchers|CreateEvent :!event Custom|OnPreGameTimerTriggered))
      (Default|RunPreAttemptStateLogic _output_get_2 2.0))))

(fn ConstructionScript)

(fn GetCurrentLevelInfo
  (return (Variables|Default|GetCurrentLevelInfo)))