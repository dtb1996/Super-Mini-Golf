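; BP_GolfPawn is the mini golf ball pawn, a physics sphere with tunable roll, tilt and hit settings.
; On BeginPlay it attaches the level's BP_GoodSky to its spring arm.
; Getter and setter functions expose the tuning values, with max angular velocity pushed straight to the sphere collision.
; It also applies impulses to the ball and forwards coin pickups to the player state.
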(event EventBeginPlay
  (|CallParentFunction)
  (bind _outactors (Actor|GetAllActorsOfClass "/Game/GoodSky/Blueprint/BP_GoodSky.BP_GoodSky_C"))
  (Utilities|IsValid (Utilities|Array|Get(acopy) _outactors)
    (:Is%20Valid
      (bind _output_get (Variables|Default|SetSkySphere (Utilities|Array|Get(acopy) _outactors)))
      (Transformation|AttachComponentToComponent _output_get (Variables|Default|GetSpringArm) "None" "KeepWorld" "KeepRelative" "KeepWorld" true))))

(fn ConstructionScript
  (|CallParentFunction))

(fn GetPawnSettings
  (return (Variables|Default|GetRollTorque) (Variables|Default|GetTiltAngularDamping) (Variables|Default|GetNormalAngularDamping) (Variables|Default|GetMaxAngularVelocity) (Variables|Default|GetTiltFactorX) (Variables|Default|GetTiltFactorY) (Variables|Default|GetHitImpulseMin) (Variables|Default|GetTiltYawInputFactorX) (Variables|Default|GetbIsTiltTurnEnabled)))

(fn SetRollTorque
  (params (RollTorque :type Float%20%28single-precision%29))
  (Variables|Default|SetRollTorque RollTorque))

(fn SetTiltAngularDamping
  (params (TiltAngularDamping :type Float%20%28single-precision%29))
  (Variables|Default|SetTiltAngularDamping TiltAngularDamping))

(fn SetNormalAngularDamping
  (params (NormalAngularDamping :type Float%20%28single-precision%29))
  (Variables|Default|SetNormalAngularDamping NormalAngularDamping))

(fn SetMaxAngularVelocity
  (params (MaxAngularVelocity :type Float%20%28single-precision%29))
  (bind _output_get (Variables|Default|SetMaxAngularVelocity MaxAngularVelocity))
  (Class|PrimitiveComponent|SetPhysicsMaxAngularVelocityinRadians (Variables|Default|GetSphereCollision) _output_get false "None"))

(fn SetTiltFactorX
  (params (TiltFactorX :type Float%20%28single-precision%29))
  (Variables|Default|SetTiltFactorX TiltFactorX))

(fn SetTiltFactorY
  (params (TiltFactorY :type Float%20%28single-precision%29))
  (Variables|Default|SetTiltFactorY TiltFactorY))

(fn SetHitImpulseMin
  (params (HitImpulseMin :type Float%20%28single-precision%29))
  (Variables|Default|SetHitImpulseMin HitImpulseMin))

(fn SetTiltYawInputX
  (params (HitImpulseMin :type Float%20%28single-precision%29))
  (Variables|Default|SetTiltYawInputFactorX HitImpulseMin))

(fn SetIsTiltTurnEnabled
  (params (IsTiltTurnEnabled :type Boolean))
  (Variables|Default|SetbIsTiltTurnEnabled IsTiltTurnEnabled))

(fn ApplyImpulse
  (params (Impulse :type Vector :default "0, 0, 0"))
  (Physics|AddImpulse (Variables|Default|GetSphereCollision) Impulse "None" false)
  (return true))

(fn CollectCoins
  (params (NumCoins :type Integer))
  (bind _success (Class|IInteract|CollectCoins(Message) (Game|GetPlayerState 0) NumCoins))
  (return _success))