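; Player state for the mini golf game that holds the player's stats, mainly score and coin count, and broadcasts changes through dispatchers.
; On BeginPlay it loads player 0's stats from the game instance and listens for game state changes, saving only the score back when the level changes.
; Collecting coins adds to the count (SetCurrentCoins is additive) and awards a flat score bonus, while ApplyImpulse is a stub returning false.
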(event Custom|OnGameStateChanged
  (params (State :type EGameStates%20Enum :default "Countdown"))
  (switch Utilities|FlowControl|Switch|SwitchonEGameStates State
    (:ChangingLevel
      (bind _gameinstanceref (Variables|Default|GetGameInstanceRef)
        (:then
          (Class|GolfGameInstance|SetPlayerScore _gameinstanceref 0 (Utilities|Struct|BreakPlayerStats (Variables|Default|GetPlayerStats))))
        (:else)))))

(event EventBeginPlay
  (Utilities|FlowControl|Sequence
    (:then_0
      (bind _asbp_golf_game_instance (Utilities|Casting|CastToBP_GolfGameInstance (Game|GetGameInstance)))
      (bind _output_get (Variables|Default|SetGameInstanceRef _asbp_golf_game_instance))
      (if (.Found (Class|GolfGameInstance|GetPlayerStats _output_get))
        (bind _output_get_2 (Variables|Default|SetPlayerStats (.ReturnValue (Class|GolfGameInstance|GetPlayerStats _output_get))))
        (Default|CallPlayerStatsUpdated _output_get_2)))
    (:then_1
      (bind _asbp_golf_game_state (Utilities|Casting|CastToBP_GolfGameState (Game|GetGameState)))
      (bind _output_get_3 (Variables|Default|SetGameStateRef _asbp_golf_game_state))
      (EventDispatchers|BindEventtoStateChanged _output_get_3 (EventDispatchers|CreateEvent :!event Custom|OnGameStateChanged)))))

(event EventDestroyed
  (bind _gamestateref (Variables|Default|GetGameStateRef)
    (:then
      (EventDispatchers|UnbindEventfromStateChanged _gamestateref (EventDispatchers|CreateEvent :!event Custom|OnGameStateChanged)))
    (:else)))

(fn ConstructionScript)

(fn GetCurrentCoins
  (return (Utilities|Struct|BreakPlayerStats (Variables|Default|GetPlayerStats))))

(fn SetCurrentCoins
  (params (InputPin :type Integer))
  (bind _structout (Utilities|Struct|SetmembersinPlayerStats (Variables|Default|GetPlayerStats) (+ InputPin (Utilities|Struct|BreakPlayerStats (Variables|Default|GetPlayerStats)))))
  (Default|CallCoinCountUpdated (Utilities|Struct|BreakPlayerStats _structout)))

(fn SetPlayerScore
  (params (NewPlayerScore :type Integer))
  (bind _structout (Utilities|Struct|SetmembersinPlayerStats (Variables|Default|GetPlayerStats) NewPlayerScore))
  (Default|CallPlayerScoreUpdated (Utilities|Struct|BreakPlayerStats _structout)))

(fn GetPlayerScore
  (return (Utilities|Struct|BreakPlayerStats (Variables|Default|GetPlayerStats))))

(fn GetPlayerStats
  (return (Variables|Default|GetPlayerStats)))

(fn SetPlayerStats
  (params (PlayerStats :type Player%20Stats%20Structure))
  (bind _output_get (Variables|Default|SetPlayerStats PlayerStats))
  (Default|CallPlayerStatsUpdated _output_get))

(fn AddtoPlayerScore
  (params (PointsToAdd :type Integer))
  (bind _playerstats (Variables|Default|GetPlayerStats))
  (bind _structout (Utilities|Struct|SetmembersinPlayerStats _playerstats (+ (Utilities|Struct|BreakPlayerStats _playerstats) PointsToAdd)))
  (Default|CallPlayerScoreUpdated (Utilities|Struct|BreakPlayerStats _structout)))

(fn ApplyImpulse
  (params (Impulse :type Vector :default "0, 0, 0"))
  (return false))

(fn CollectCoins
  (params (NumCoins :type Integer))
  (CallFunction|SetCurrentCoins NumCoins)
  (CallFunction|SetPlayerScore (+ (CallFunction|GetPlayerScore) 50))
  (return true))