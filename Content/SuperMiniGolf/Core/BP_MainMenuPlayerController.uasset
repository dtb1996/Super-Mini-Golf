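; Player controller for the main menu that switches cursor display between gamepad and mouse input.
; On BeginPlay it adds the menu input mapping context and binds to the GolfGameInstance's input-hardware-changed event.
; Each hardware change hides the cursor for gamepads, shows it otherwise, and reapplies Game and UI input with the mouse locked.
; Destroyed also calls the bind function, rather than an unbind.
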(event Custom|OnInputHardwareChanged
  (params (IsGamepad :type Boolean))
  (Variables|Default|SetbShowMouseCursor (not IsGamepad))
  (Input|SetInputModeGameandUI self 0 "LockAlways" false true))

(event EventBeginPlay
  (Input|AddMappingContext (PlayerController|LocalPlayerSubsystems|GetEnhancedInputLocalPlayerSubsystem self) "/Game/SuperMiniGolf/Core/Input/IMC_Menu.IMC_Menu" 0 "(bIgnoreAllPressedKeysUntilRelease=True,bForceImmediately=False,bNotifyUserSettings=False)")
  (bind _asgolf_game_instance (Utilities|Casting|CastToGolfGameInstance (Game|GetGameInstance)))
  (bind _output_get (Variables|Default|SetGameInstanceRef _asgolf_game_instance))
  (EventDispatchers|BindEventtoOnInputHardwareChanged _output_get (EventDispatchers|CreateEvent :!event Custom|OnInputHardwareChanged)))

(event EventDestroyed
  (bind _gameinstanceref (Variables|Default|GetGameInstanceRef)
    (:then
      (EventDispatchers|BindEventtoOnInputHardwareChanged _gameinstanceref (EventDispatchers|CreateEvent :!event Custom|OnInputHardwareChanged)))
    (:else)))

(fn ConstructionScript)